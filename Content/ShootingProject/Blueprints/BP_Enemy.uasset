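; BP_Enemy is an enemy actor for a shooting game that flies in a straight line and collides with the player.
; On BeginPlay it randomly, based on TraceRate, aims once at the BP_PlayerPawn's position, otherwise it uses its forward vector.
; Tick moves it along that fixed Direction by MoveSpeed scaled by delta time, without sweep.
; Overlapping the player pawn destroys both actors and spawns an explosion emitter.
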(event `self.ReceiveActorBeginOverlap`
  (params (OtherActor :type "Actor Object Reference"))
  (bind _asbp_player_pawn (cast `/Game/ShootingProject/Blueprints/BP_PlayerPawn` OtherActor))
  (`self.K2_DestroyActor` _asbp_player_pawn)
  (`GameplayStatics.SpawnEmitterAtLocation` "/Game/StarterContent/Particles/P_Explosion.P_Explosion" (`self.K2_GetActorLocation`))
  (`self.K2_DestroyActor`))

(event `self.ReceiveBeginPlay`
  (if (<= (`KismetMathLibrary.RandomFloatInRange` 0.0 1.0) (`self.TraceRate`))
    ;[1 1 1] 월드에 있는 선택한 클래스 인스턴스를 반환한다.
    (bind _returnvalue (`GameplayStatics.GetActorOfClass` "/Game/ShootingProject/Blueprints/BP_PlayerPawn.BP_PlayerPawn_C"))
    ;[1 1 1] 들어 온 값이 유효한 지 체크해준다.
    (`/Engine/EditorBlueprintResources/StandardMacros.IsValid` _returnvalue
      (:`Is Valid`
        (set `self.Direction` (`KismetMathLibrary.Normal` (- (`self.K2_GetActorLocation` _returnvalue) (`self.K2_GetActorLocation`)))))
      (:`Is Not Valid`
        (set `self.Direction` (`self.GetActorForwardVector`))))
    (else
      (set `self.Direction` (`self.GetActorForwardVector`)))))

(event `self.ReceiveTick`
  (params (DeltaSeconds :type "Float (single-precision)"))
  ;[1 1 1] 들어온 좌표로 액터를  순간 이동시킨다.
  (`self.K2_SetActorLocation` (+ (`self.K2_GetActorLocation`) (* DeltaSeconds (* (`self.Direction`) (`self.MoveSpeed`))))))

(fn `UserConstructionScript`)