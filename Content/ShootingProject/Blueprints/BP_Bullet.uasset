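; BP_Bullet is a projectile actor for a shooting game that destroys enemies and awards score on contact.
; Tick moves it along its forward vector at MoveSpeed, scaled by delta time, setting location directly without sweeping.
; Overlapping a BP_Enemy destroys that enemy, spawns an explosion at the bullet, adds a point through BP_GameModeBase, then destroys the bullet.
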(event `self.ReceiveActorBeginOverlap`
  (params (OtherActor :type "Actor Object Reference"))
  ;[1 1 1] 엑터가 오버랩을 시작할 때
  (bind _asbp_enemy (cast `/Game/ShootingProject/Blueprints/BP_Enemy` OtherActor))
  (`self.K2_DestroyActor` _asbp_enemy)
  (`GameplayStatics.SpawnEmitterAtLocation` "/Game/StarterContent/Particles/P_Explosion.P_Explosion" (`self.K2_GetActorLocation`))
  (bind _asbp_game_mode_base (cast `/Game/ShootingProject/Blueprints/BP_GameModeBase` (`GameplayStatics.GetGameMode`)))
  (`/Game/ShootingProject/Blueprints/BP_GameModeBase.AddScore` _asbp_game_mode_base 1)
  (`self.K2_DestroyActor`))

(event `self.ReceiveTick`
  (params (DeltaSeconds :type "Float (single-precision)"))
  ;[1 1 1] 들어온 좌표로 액터를  순간 이동시킨다.
  (`self.K2_SetActorLocation` (+ (`self.K2_GetActorLocation`) (* DeltaSeconds (* (`self.GetActorForwardVector`) (`self.MoveSpeed`))))))

(fn `UserConstructionScript`)