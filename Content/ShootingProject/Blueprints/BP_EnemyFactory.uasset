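; BP_EnemyFactory is a spawner actor that repeatedly creates BP_Enemy actors at random intervals.
; BeginPlay picks a random initial delay, and Tick accumulates elapsed time until that delay is reached.
; It then spawns an enemy at the SpawnPoint component's world transform, resets the timer, and rolls a new random delay.
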(event `self.ReceiveBeginPlay`
  (set `self.DelayTime` (`KismetMathLibrary.RandomFloatInRange` 1.0 3.5)))

(event `self.ReceiveTick`
  (params (DeltaSeconds :type "Float (single-precision)"))
  (bind _output_get (set `self.CurrentTime` (+ DeltaSeconds (`self.CurrentTime`))))
  (if (>= _output_get (`self.DelayTime`))
    (`|SpawnActorFromClass` "/Game/ShootingProject/Blueprints/BP_Enemy.BP_Enemy_C" (`SceneComponent.K2_GetComponentToWorld` (`self.SpawnPoint`)) "Undefined" "MultiplyWithRoot" null null)
    (set `self.CurrentTime` 0.0)
    (set `self.DelayTime` (`KismetMathLibrary.RandomFloatInRange` 1.0 3.5))))

(fn `UserConstructionScript`)