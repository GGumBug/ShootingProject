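; BP_PlayerPawn is the player-controlled pawn of a shooting project, moving on the YZ plane and firing bullets.
; BeginPlay adds the IMC_PlayerInput Enhanced Input context, and horizontal and vertical actions store their axis values.
; Tick normalizes those values and moves the pawn by MoveSpeed scaled by delta time, without sweeping for collision.
; The fire action spawns BP_Bullet at the FireArrow transform and plays a 2D blaster sound.
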(event `self.ReceiveBeginPlay`
  ;[1 1 1] 입력 매핑을 플레이어에게 적용한다.
  (`EnhancedInputSubsystemInterface.AddMappingContext` (pcsubsystem `EnhancedInputLocalPlayerSubsystem` (`GameplayStatics.GetPlayerController` 0)) "/Game/ShootingProject/Inputs/IMC_PlayerInput.IMC_PlayerInput" 0 (struct)))

(event `EnhancedInput|/Game/ShootingProject/Inputs/IA_Horizontal`
  (params (ActionValue :type "Float (double-precision)") (ElapsedSeconds :type "Float (double-precision)") (TriggeredSeconds :type "Float (double-precision)") (InputAction :type "InputAction Object Reference" :default "/Game/ShootingProject/Inputs/IA_Horizontal.IA_Horizontal"))
  (:`Triggered`
    (set `self.Horizontal` ActionValue))
  (:`Completed`
    (set `self.Horizontal` ActionValue)))

(event `EnhancedInput|/Game/ShootingProject/Inputs/IA_Fire`
  (params (ActionValue :type Boolean) (ElapsedSeconds :type "Float (double-precision)") (TriggeredSeconds :type "Float (double-precision)") (InputAction :type "InputAction Object Reference" :default "/Game/ShootingProject/Inputs/IA_Fire.IA_Fire"))
  ;[1 1 1] 왼쪽 클릭을 할 때 신호가 들어오는 이벤트 노드
  (:`Started`
    ;[1 1 1] 월드에 엑터를 스폰 시키는데, 내가 설정한 클래스의 엑터를 스폰시킨다.
    (`|SpawnActorFromClass` "/Game/ShootingProject/Blueprints/BP_Bullet.BP_Bullet_C" (`SceneComponent.K2_GetComponentToWorld` (`self.Fire Arrow`)) "Undefined" "MultiplyWithRoot" null null)
    ;[1 1 1] 거리에 상관없는 2D 사운드가 재생 된다.
    (`GameplayStatics.PlaySound2D` "/Game/ShootingProject/Audio/star-wars-blaster.star-wars-blaster" 1.0 1.0 0.0 null null)))

(event `EnhancedInput|/Game/ShootingProject/Inputs/IA_Vertical`
  (params (ActionValue :type "Float (double-precision)") (ElapsedSeconds :type "Float (double-precision)") (TriggeredSeconds :type "Float (double-precision)") (InputAction :type "InputAction Object Reference" :default "/Game/ShootingProject/Inputs/IA_Vertical.IA_Vertical"))
  (:`Triggered`
    (set `self.Vertical` ActionValue))
  (:`Completed`
    (set `self.Vertical` ActionValue)))

(event `self.ReceiveTick`
  (params (DeltaSeconds :type "Float (single-precision)"))
  ;[1 1 1] 매 프레임마다 실행
  ;[1 1 1] 들어온 벡터 값대로 내 위치를 바꾼다.
  (`self.K2_SetActorLocation` (+ (`self.K2_GetActorLocation`) (* DeltaSeconds (* (`KismetMathLibrary.Normal` (`KismetMathLibrary.MakeVector` 0.0 (`self.Horizontal`) (`self.Vertical`))) (`self.MoveSpeed`))))))

(fn `UserConstructionScript`)